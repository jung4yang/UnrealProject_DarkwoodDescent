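; BP_Door is an interactable hinged door that opens and closes on each Interact event.
; An open-state flag picks whether to play or reverse a Timeline, with a creak sound for each direction at the door's location.
; The Timeline alpha drives the Hinge's relative yaw through a quarter turn.
; GetInteractPrompt always returns "Open the door", regardless of the door's state.
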(event `/Game/DarkwoodDescent/Blueprints/BPI_Interactable.Interact`
  (params (Caller :type "Actor Object Reference"))
  (bind _returnvalue (`self.K2_GetActorLocation`))
  (if (`self.bisOpen`)
    (`GameplayStatics.PlaySoundAtLocation` "/Game/DarkwoodDescent/Audio/CloseDoorCreek.CloseDoorCreek" _returnvalue (struct) 1.0 1.0 0.0 null null null null)
    (set `self.bisOpen` false)
    (bind (_direction _alpha) (`Timeline|Timeline` :!via `Reverse` :!label _label)
      (:`Update`
        (`SceneComponent.K2_SetRelativeRotation` (`self.Hinge`) (`KismetMathLibrary.MakeRotator` 0.0 0.0 (`KismetMathLibrary.Lerp` 0.0 90.0 _alpha)) false false)
        (`/Engine/EditorBlueprintResources/StandardMacros.DoOnce` false)))
    (else
      (`GameplayStatics.PlaySoundAtLocation` "/Game/DarkwoodDescent/Audio/OpenDoorCreekl.OpenDoorCreekl" _returnvalue (struct) 1.0 1.0 0.0 null null null null)
      (set `self.bisOpen` true)
      (goto _label))))

(event `GetInteractPrompt_1_1`)

(fn `GetInteractPrompt`
  (returns (Text :type Text))
  (return "Open the door"))

(fn `UserConstructionScript`)